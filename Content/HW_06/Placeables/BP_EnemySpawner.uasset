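; Placeable enemy spawner that periodically spawns a random NPC class from Types while its count of living enemies is below Limit.
; A looping timer calls SpawnNewEnemy, which picks a random XY inside the Box at root height, faces the Arrow's direction and skips blocked spots it cannot adjust.
; Spawned enemies are tracked in an array and removed through their death dispatcher, freeing slots for later ticks.
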(event `self.ReceiveBeginPlay`
  (`KismetSystemLibrary.K2_SetTimerDelegate` (delegate `OnSpawnTimerTick`) (`self.Time`) true))

(event `OnSpawnTimerTick`
  (bind (_success _newenemy) (`self.SpawnNewEnemy`))
  (if _success
    (`KismetArrayLibrary.Array_Add` (`self.SpawnedEnemies`) _newenemy)
    (add `/Game/HW_06/Characters/BP_BaseCharacter.OnDeathDispatcher` _newenemy (delegate `OnSpawnedEnemyDied`))))

(event `OnSpawnedEnemyDied`
  (params (EnemyCharacter :type "/Game/HW_06/Characters/BP_BaseCharacter Object Reference"))
  (bind _asbp_npc_character (cast `/Game/HW_06/Characters/BP_NpcCharacter` EnemyCharacter))
  (`KismetArrayLibrary.Array_RemoveItem` (`self.SpawnedEnemies`) _asbp_npc_character)
  (remove `/Game/HW_06/Characters/BP_BaseCharacter.OnDeathDispatcher` _asbp_npc_character (delegate `OnSpawnedEnemyDied`)))

(fn `SpawnNewEnemy`
  (returns (Success :type Boolean) (NewEnemy :type "/Game/HW_06/Characters/BP_NpcCharacter Object Reference"))
  (bind _returnvalue (`SceneComponent.K2_GetComponentLocation` (`self.DefaultSceneRoot`)))
  (bind (_returnvalue_x _returnvalue_y) (`KismetMathLibrary.BreakVector` (`KismetMathLibrary.RandomPointInBoundingBox` _returnvalue (`BoxComponent.GetScaledBoxExtent` (`self.Box`)))))
  (if (and (< (`KismetArrayLibrary.Array_Length` (`self.SpawnedEnemies`)) (`self.Limit`)) (`KismetArrayLibrary.Array_IsNotEmpty` (`self.Types`)))
    (bind _returnvalue_2 (`|SpawnActorFromClass` (`KismetArrayLibrary.Array_Random` (`self.Types`)) (`KismetMathLibrary.MakeTransform` (`KismetMathLibrary.MakeVector` _returnvalue_x _returnvalue_y (.z _returnvalue)) (`SceneComponent.K2_GetComponentRotation` (`self.Arrow`))) "AdjustIfPossibleButDontSpawnIfColliding" "MultiplyWithRoot" null null))
    (`/Engine/EditorBlueprintResources/StandardMacros.IsValid` _returnvalue_2
      (:`Is Valid`
        (return true _returnvalue_2))
      (:`Is Not Valid`
        (return false null)))
    (else
      (return false null))))

(fn `UserConstructionScript`)