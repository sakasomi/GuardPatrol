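; Gameplay ability that makes an NPC fire projectiles repeatedly while its blackboard flags the player as detected.
; Each committed activation plays the shooting montage and fires at its start, looping on montage completion or blend-out.
; Shots trace along the actor's forward vector, then spawn a muzzle projectile aimed at the hit or range limit.
; Each shot applies GE_Shoot to the owner; ability end removes effects tagged Effect.Ability.Shoot.
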(event `self.K2_ActivateAbility`
  (bind _returnvalue (`self.GetAvatarActorFromActorInfo`))
  (`/Engine/EditorBlueprintResources/StandardMacros.IsValid` _returnvalue
    (:`Is Valid`
      (bind _asbp_npc_character (cast `/Game/HW_06/Characters/BP_NpcCharacter` _returnvalue)
        (:`then`
          (set `self.NpcCharacter` _asbp_npc_character)
          (bind _returnvalue_2 (`self.K2_CommitAbility` :!label _label))
          (if _returnvalue_2
            (`AbilityTask_PlayMontageAndWait.CreatePlayMontageAndWaitProxy` "None" "/Game/HW_06/Animations/Guard/AM_Shooting.AM_Shooting" 0.5
              (:`then`
                (`self.Shoot`))
              (:`OnCompleted`
                (if (`BlackboardComponent.GetValueAsBool` (`AIBlueprintHelperLibrary.GetBlackboard` (`self.NpcCharacter`)) "PlayerDetected") :!label _label_2
                  (goto _label)
                  (else
                    (`self.K2_EndAbility`))))
              (:`OnBlendOut`
                (goto _label_2))
              (:`OnInterrupted`
                (`self.K2_CancelAbility` :!label _label_3))
              (:`OnCancelled`
                (goto _label_3)))
            (else
              (`self.K2_EndAbility`))))
        (:`CastFailed`
          (`self.K2_CancelAbility` :!label _label_4))))
    (:`Is Not Valid`
      (goto _label_4))))

(event `self.K2_OnEndAbility`
  (params (bWasCancelled :type Boolean))
  (`self.BP_RemoveGameplayEffectFromOwnerWithAssetTags` (struct :`GameplayTags` (struct :`(TagName` "Effect.Ability.Shoot") :`(TagName` "Status.Character.Ability.Shoot")))))

(fn `Shoot`
  (bind _npccharacter (`self.NpcCharacter`))
  (bind _returnvalue (`Actor.K2_GetActorLocation` _npccharacter))
  (bind _returnvalue_2 (`SceneComponent.GetSocketLocation` (`/Game/HW_06/Characters/BP_NpcCharacter.WeaponMesh` (`self.NpcCharacter`)) "Muzzle"))
  (bind _returnvalue_3 (+ _returnvalue (* (`Actor.GetActorForwardVector` _npccharacter) 2000.0)))
  (bind _outhit (`KismetSystemLibrary.LineTraceSingle` _returnvalue _returnvalue_3 "TraceTypeQuery1"))
  (bind (_bblockinghit _binitialoverlap _time _distance _location) (`GameplayStatics.BreakHitResult` _outhit))
  (`|SpawnActorFromClass` "/Game/FirstPerson/Blueprints/BP_FirstPersonProjectile.BP_FirstPersonProjectile_C" (`KismetMathLibrary.MakeTransform` _returnvalue_2 (`KismetMathLibrary.FindLookAtRotation` _returnvalue_2 (`KismetMathLibrary.SelectVector` _location _returnvalue_3 _bblockinghit)) (0.3 0.3 0.3)) "Undefined" "MultiplyWithRoot" null null)
  (`self.BP_ApplyGameplayEffectToOwner` "/Game/HW_06/GameSystem/GameplayAbilities/Shoot/GE_Shoot.GE_Shoot_C"))