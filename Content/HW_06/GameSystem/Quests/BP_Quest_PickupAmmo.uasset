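; BP_Quest_PickupAmmo is a quest that completes once the player picks up every tagged pickup in the level.
; On activation it finds all BP_Pickup actors with its item tag, records their count, activates each and binds to its OnPickup event.
; Each pickup increments a counter, and the quest marks itself completed when the counter matches the total.
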(event `self.ActivateQuest`
  (bind _outactors (`GameplayStatics.GetAllActorsOfClassWithTag` "/Game/HW_06/GameSystem/Quests/BP_Pickup.BP_Pickup_C" (`self.ItemTag`)))
  (set `self.NumberOfItemsToPickup` (`KismetArrayLibrary.Array_Length` _outactors))
  (for _array_element _outactors
    (`/Game/HW_06/GameSystem/Quests/BP_Pickup.Activate` _array_element)
    (add `/Game/HW_06/GameSystem/Quests/BP_Pickup.OnPickup` _array_element (delegate `OnItemPickedUp`))))

(event `OnItemPickedUp`
  (`/Engine/EditorBlueprintResources/StandardMacros.IncrementInt` (`self.PickedUpCount`)
    (:`  `
      (if (== (`self.NumberOfItemsToPickup`) (`self.PickedUpCount`))
        (`self.SetIsCompleted` true)))))

(fn `UserConstructionScript`
  (`parent.UserConstructionScript`))