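; BP_QuestManager runs the level's quests one after another in order of their quest number.
; On BeginPlay it collects every BP_Quest actor into a map keyed by quest number, then activates the quest matching CurrentQuestNumber.
; It listens for that quest's completion, then unbinds, increments the number and activates the next.
; When a number has no quest, it prints a message instead.
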(event `self.ReceiveBeginPlay`
  (bind _outactors (`GameplayStatics.GetAllActorsOfClass` "/Game/HW_06/GameSystem/Quests/BP_Quest.BP_Quest_C"))
  (for _array_element _outactors
    (`BlueprintMapLibrary.Map_Add` (`self.Quests`) (`/Game/HW_06/GameSystem/Quests/BP_Quest.GetQuestNumber` _array_element) _array_element))
  (bind (_isfound _value) (`self.TryGetQuestByNumber` (`self.CurrentQuestNumber`)))
  (if _isfound
    (`/Game/HW_06/GameSystem/Quests/BP_Quest.ActivateQuest` _value)
    (add `/Game/HW_06/GameSystem/Quests/BP_Quest.OnQuestCompleted` _value (delegate `OnCurrentQuestCompleted`))))

(event `OnCurrentQuestCompleted`
  (params (Source :type "/Game/HW_06/GameSystem/Quests/BP_Quest Object Reference"))
  (remove `/Game/HW_06/GameSystem/Quests/BP_Quest.OnQuestCompleted` Source (delegate `OnCurrentQuestCompleted`))
  (`/Engine/EditorBlueprintResources/StandardMacros.IncrementInt` (`self.CurrentQuestNumber`)
    (:`  `
      (bind (_isfound _value) (`self.TryGetQuestByNumber` (`self.CurrentQuestNumber`)))
      (if _isfound
        (`/Game/HW_06/GameSystem/Quests/BP_Quest.ActivateQuest` _value)
        (add `/Game/HW_06/GameSystem/Quests/BP_Quest.OnQuestCompleted` _value (delegate `OnCurrentQuestCompleted`))
        (else
          (`KismetSystemLibrary.PrintString` "Больше квестов не существует"))))))

(fn `TryGetQuestByNumber`
  (params (Number :type Integer))
  (returns (IsFound :type Boolean) (Value :type "/Game/HW_06/GameSystem/Quests/BP_Quest Object Reference"))
  (bind (_value _returnvalue) (`BlueprintMapLibrary.Map_Find` (`self.Quests`) Number))
  (if _returnvalue
    (return _returnvalue _value)
    (else
      (`KismetSystemLibrary.PrintString` (`KismetTextLibrary.Conv_TextToString` (`|FormatText` "Не удается найти квест номер: {1}" Number))))))

(fn `UserConstructionScript`)