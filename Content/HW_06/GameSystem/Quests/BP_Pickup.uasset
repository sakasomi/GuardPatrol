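; BP_Pickup is an ammo pickup in the quest system that adds 15 rounds to the player's ammo bag on overlap.
; Activate makes its static mesh visible and turns on overlap events; the logic that would hide and disable it is unconnected.
; When a BP_BasePlayerCharacter overlaps the mesh, it fires OnPickup, unbinds all its listeners, grants the ammo, prints a Russian message and destroys itself.
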(event `self.ReceiveBeginPlay`)

(event `Activate`
  (set `PrimitiveComponent.bGenerateOverlapEvents` true (`self.StaticMesh`))
  (`SceneComponent.SetVisibility` (`self.StaticMesh`) true false))

(event `self.StaticMesh.OnComponentBeginOverlap`
  (params (OverlappedComponent :type "PrimitiveComponent Object Reference") (OtherActor :type "Actor Object Reference") (OtherComp :type "PrimitiveComponent Object Reference") (OtherBodyIndex :type Integer) (bFromSweep :type Boolean) (SweepResult :type "HitResult Structure (by ref)"))
  (bind _asbp_base_player_character (cast `/Game/HW_06/Characters/BP_BasePlayerCharacter` OtherActor))
  (`/Engine/EditorBlueprintResources/StandardMacros.IsValid` _asbp_base_player_character
    (:`Is Valid`
      (`self.OnPickup`)
      (clear `self.OnPickup`)
      (set `/Game/HW_06/Characters/BP_BasePlayerCharacter.AmmoBag` (+ (`/Game/HW_06/Characters/BP_BasePlayerCharacter.AmmoBag` _asbp_base_player_character) 15) _asbp_base_player_character)
      (`KismetSystemLibrary.PrintString` "Вы подобрали 15 патронов.")
      (`self.K2_DestroyActor`))))

(fn `UserConstructionScript`
  (`parent.UserConstructionScript`))