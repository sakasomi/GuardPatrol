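; BP_Quest is a quest object that holds a number, a name and a completion flag, exposed through getter and setter functions.
; SetIsCompleted calls the OnQuestCompleted dispatcher with itself only when the flag changes from false to true, broadcasting before the new value is stored.
; ActivateQuest is an empty event, and this Blueprint contains no objective logic of its own.
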(event `ActivateQuest`)

(fn `GetIsCompleted`
  (returns (IsCompleted :type Boolean))
  (return (`self.IsCompleted`)))

(fn `GetQuestName`
  (returns (Name :type Text))
  (return (`self.Name`)))

(fn `GetQuestNumber`
  (returns (Number :type Integer))
  (return (`self.Number`)))

(fn `Set Quest Name`
  (params (NewName :type Text))
  (set `self.Name` NewName))

(fn `SetIsCompleted`
  (params (NewIsCompleted :type Boolean))
  (if (and NewIsCompleted (not (`self.IsCompleted`)))
    (if true
      (`self.OnQuestCompleted` self)
      (set `self.IsCompleted` (`local.NewIsCompleted`) :!label _label))
    (else
      (goto _label))))

(fn `SetQuestNumber`
  (params (NewNumber :type Integer))
  (set `self.Number` NewNumber))

(fn `UserConstructionScript`)