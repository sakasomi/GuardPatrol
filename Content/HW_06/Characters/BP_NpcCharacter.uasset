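; BP_NpcCharacter is an NPC character that can use a shoot ability and shows a health bar above its head.
; On BeginPlay it runs the parent logic, then grants GA_Shoot through its Ability System component.
; It then casts its widget component's widget to WBP_HealthBar and sets itself as that widget's owner reference.
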(event `self.ReceiveBeginPlay`
  (`parent.ReceiveBeginPlay`)
  (`|ExecutionSequence`
    (:`then_0`
      (`AbilitySystemComponent.K2_GiveAbility` (`self.AbilitySystem`) "/Game/HW_06/GameplayAbilities/Shoot/GA_Shoot.GA_Shoot_C" 0 1))
    (:`then_1`
      ;[1 1 1] Здоровье над головой персонажа
      (bind _aswbp_health_bar (cast `/Game/HW_06/UI/WBP_HealthBar` (`WidgetComponent.GetWidget` (`self.Widget`))))
      (set `/Game/HW_06/UI/WBP_HealthBar.WidgetOwner` self _aswbp_health_bar))))

(fn `UserConstructionScript`
  (`parent.UserConstructionScript`))