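; Base character Blueprint using the Gameplay Ability System, handling projectile damage and death for players and other characters.
; An async task watches an attribute and triggers death at zero or below, printing a message for player characters.
; Capsule overlaps with first-person projectiles apply a damage effect.
; Death applies its own effect, fires a dispatcher, clears physical animation, ragdolls the mesh, disables capsule collision and destroys the actor after a delay.
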(event `self.ReceiveBeginPlay`
  (bind (_asynctaskproxy _attribute _newvalue) (`AbilityAsync_WaitAttributeChanged.WaitForAttributeChanged` null (struct :`AttributeName` "Health" :`Attribute` "/Script/HW_06.CharacterAttributeSet:Health" :`AttributeOwner` "/Script/CoreUObject.Class'/Script/HW_06.CharacterAttributeSet'"))
    (:`Changed`
      (if (<= _newvalue 0.0)
        (if (`GameplayStatics.ObjectIsA` self "/Game/HW_06/Characters/BP_BasePlayerCharacter.BP_BasePlayerCharacter_C")
          (`KismetSystemLibrary.PrintText` "Персонаж погиб.")
          (`CancellableAsyncAction.Cancel` _asynctaskproxy)
          (`self.OnDeath`)
          (else
            (`CancellableAsyncAction.Cancel` _asynctaskproxy)
            (`self.OnDeath`)))))))

(event `OnDeath`
  (bind _capsulecomponent (`self.CapsuleComponent`))
  (`AbilitySystemComponent.BP_ApplyGameplayEffectToSelf` :`self` (`self.AbilitySystem`) :`GameplayEffectClass` "/Game/HW_06/GameSystem/GameplayAbilities/PassiveEffects/GE_Death.GE_Death_C")
  (`self.OnDeathDispatcher` self)
  (`self.DisablePA`)
  (`self.EnableRagdoll` (`self.RagdollRootBone`))
  (`PrimitiveComponent.SetCollisionEnabled` _capsulecomponent "NoCollision")
  (set `PrimitiveComponent.bGenerateOverlapEvents` false _capsulecomponent)
  (`KismetSystemLibrary.Delay` 2.0)
  (`self.K2_DestroyActor`))

(event `self.CapsuleComponent.OnComponentBeginOverlap`
  (params (OverlappedComponent :type "PrimitiveComponent Object Reference") (OtherActor :type "Actor Object Reference") (OtherComp :type "PrimitiveComponent Object Reference") (OtherBodyIndex :type Integer) (bFromSweep :type Boolean) (SweepResult :type "HitResult Structure (by ref)"))
  (`/Engine/EditorBlueprintResources/StandardMacros.IsValid` OtherActor
    (:`Is Valid`
      (cast `/Game/FirstPerson/Blueprints/BP_FirstPersonProjectile` OtherActor)
      (`AbilitySystemComponent.BP_ApplyGameplayEffectToSelf` :`self` (`self.AbilitySystem`) :`GameplayEffectClass` "/Game/HW_06/GameSystem/GameplayAbilities/Shoot/GE_ShootDamage.GE_ShootDamage_C"))))

(fn `DisablePA`
  (`PhysicalAnimationComponent.SetSkeletalMeshComponent` (`self.PhysicalAnimation`) null))

(fn `EnableRagdoll`
  (params (InBoneName :type Name))
  (locals (InitialTransform :type "Transform Structure"))
  (`PrimitiveComponent.SetCollisionProfileName` (`self.Mesh`) "Ragdoll" true)
  (`SkeletalMeshComponent.SetAllBodiesBelowSimulatePhysics` (`self.Mesh`) InBoneName true true)
  (`CharacterMovementComponent.DisableMovement` (`self.CharacterMovement`))
  (return))

(fn `UserConstructionScript`)